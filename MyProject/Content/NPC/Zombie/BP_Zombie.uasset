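; BP_Zombie is a zombie NPC driven by an enum state switch in UpdateStateOfZombie, each state playing its own animation.
; Idle polls for a path to the player, running chases via AI MoveTo, and success triggers a timed attack before chasing again.
; BeginPlay enters Death, which plays a sound and enables physics.
; Idle's range check subtracts the player's location from itself, so any valid path starts the chase.
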(event Custom|UpdateStateOfZombie
  (params (ActualStateOfZombie :type Enum_Anim_Zombie%20Enum :default "NewEnumerator0"))
  (bind _returnvalue (Game|GetPlayerCharacter 0))
  ;[1 0.782 0] Switch On and Beginplay
  (bind _output_get (Variables|Default|SetActualStateOfZombie ActualStateOfZombie))
  (switch Utilities|FlowControl|Switch|SwitchonEnum_Anim_Zombie _output_get
    (:NewEnumerator1
      ;[0.2922 0 1] Idle_Anim_Zombie
      (Components|Animation|PlayAnimation (Variables|Default|GetSkeletalMesh) "/Game/NPC/Zombie/TexturesAndObjects/AnimationsZombie/Idle_Anim_Zombie.Idle_Anim_Zombie" true)
      (bind _returnvalue_2 (Class|NavigationSystemV1|FindPathtoActorSynchronously (Transformation|GetActorLocation) (Game|GetPlayerCharacter 0) 5e+01 0 0 :!label _label))
      (if (not (Utilities|IsValid _returnvalue_2))
        (Utilities|FlowControl|Delay 0.2 :!label _label_2)
        (goto _label)
        (elif (< (Math|Vector|VectorLengthXY (- (Transformation|GetActorLocation _returnvalue) (Transformation|GetActorLocation _returnvalue))) 5e+02)
          (CallFunction|UpdateStateOfZombie "NewEnumerator4")
          (else
            (goto _label_2)))))
    (:NewEnumerator3
      ;[0.261 0.526 0.2438] Hit the Player (Zombie Attack)
      (Components|Animation|PlayAnimation (Variables|Default|GetSkeletalMesh) "/Game/NPC/Zombie/TexturesAndObjects/AnimationsZombie/HitPlayer_Anim_Zombie.HitPlayer_Anim_Zombie" false)
      (Utilities|FlowControl|Delay 2.63)
      (CallFunction|UpdateStateOfZombie "NewEnumerator4"))
    (:NewEnumerator4
      ;[0 0.6968 1] Zombie is following the player
      (Components|Animation|PlayAnimation (Variables|Default|GetSkeletalMesh) "/Game/NPC/Zombie/TexturesAndObjects/AnimationsZombie/SlowRun_Anim_Zombie.SlowRun_Anim_Zombie" true)
      (AI|AIMoveTo self "0, 0, 0" (Game|GetPlayerCharacter 0) 5.0 false
        (:OnSuccess
          (CallFunction|UpdateStateOfZombie "NewEnumerator3"))
        (:OnFail
          (CallFunction|UpdateStateOfZombie "NewEnumerator1"))))
    (:NewEnumerator5
      (Components|Animation|PlayAnimation (Variables|Default|GetSkeletalMesh) "/Game/NPC/Zombie/TexturesAndObjects/AnimationsZombie/Death_Anim_Zombie.Death_Anim_Zombie" false)
      (Utilities|FlowControl|Sequence
        (:then_0
          (Audio|PlaySound2D 0 1.0 1.0 0.0 0 0))
        (:then_1
          (Physics|SetSimulatePhysics (Variables|Default|GetTarget) true))))
    (:NewEnumerator6
      (Components|Animation|PlayAnimation (Variables|Default|GetSkeletalMesh) "/Game/NPC/Zombie/TexturesAndObjects/AnimationsZombie/Agony_Anim_Zombie.Agony_Anim_Zombie" false))))

(event EventBeginPlay
  ;[1 0.782 0] Switch On and Beginplay
  (CallFunction|UpdateStateOfZombie "NewEnumerator5"))

(event Collision|EventActorBeginOverlap
  (params (OtherActor :type Actor%20Object%20Reference)))

(event EventTick
  (params (DeltaSeconds :type Float%20%28single-precision%29)))

(event Collision|EventHit
  (params (MyComp :type Primitive%20Component%20Object%20Reference) (Other :type Actor%20Object%20Reference) (OtherComp :type Primitive%20Component%20Object%20Reference) (bSelfMoved :type Boolean) (HitLocation :type Vector :default "0, 0, 0") (HitNormal :type Vector :default "0, 0, 0") (NormalImpulse :type Vector :default "0, 0, 0") (Hit :type Hit%20Result%20Structure%20%28by%20ref%29)))

(fn ConstructionScript)