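; BP_Bullet is a projectile Blueprint that deals damage on hit to mines, zombies and the exterminator boss.
; Its Hit event runs a Sequence with one cast per target class, applying the Damage variable when a cast succeeds.
; The branches share a tail that spawns a Niagara spark effect along the hit normal and destroys the bullet, which the mine branch reaches on any hit.
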(event OnComponentBeginOverlap(SphereColision)
  (params (OverlappedComponent :type Primitive%20Component%20Object%20Reference) (OtherActor :type Actor%20Object%20Reference) (OtherComp :type Primitive%20Component%20Object%20Reference) (OtherBodyIndex :type Integer) (bFromSweep :type Boolean) (SweepResult :type Hit%20Result%20Structure%20%28by%20ref%29)))

(event OnComponentHit(SphereColision)
  (params (HitComponent :type Primitive%20Component%20Object%20Reference) (OtherActor :type Actor%20Object%20Reference) (OtherComp :type Primitive%20Component%20Object%20Reference) (NormalImpulse :type Vector :default "0, 0, 0") (Hit :type Hit%20Result%20Structure%20%28by%20ref%29)))

(event EventBeginPlay)

(event Collision|EventActorBeginOverlap
  (params (OtherActor :type Actor%20Object%20Reference)))

(event EventTick
  (params (DeltaSeconds :type Float%20%28single-precision%29)))

(event Collision|EventHit
  (params (MyComp :type Primitive%20Component%20Object%20Reference) (Other :type Actor%20Object%20Reference) (OtherComp :type Primitive%20Component%20Object%20Reference) (bSelfMoved :type Boolean) (HitLocation :type Vector :default "0, 0, 0") (HitNormal :type Vector :default "0, 0, 0") (NormalImpulse :type Vector :default "0, 0, 0") (Hit :type Hit%20Result%20Structure%20%28by%20ref%29))
  (Utilities|FlowControl|Sequence
    (:then_0
      (bind _asbp_mine (Utilities|Casting|CastToBP_Mine Other)
        (:then
          (Game|Damage|ApplyDamage _asbp_mine (Variables|Default|GetDamage) 0 0))
        (:CastFailed
          _)))
    (:then_1
      (bind _asbp_zombiee (Utilities|Casting|CastToBP_Zombiee Other))
      (Game|Damage|ApplyDamage _asbp_zombiee (Variables|Default|GetDamage) 0 0))
    (:then_2
      (bind _asboss_exterminator (Utilities|Casting|CastToBOSS_exterminator Other))
      (Game|Damage|ApplyDamage _asboss_exterminator (Variables|Default|GetDamage) 0 0)))
  (Niagara|SpawnSystematLocation "/Game/Carpeta_De_Gero/VFX/VFX_Sparks.VFX_Sparks" HitLocation (Math|Conversions|RotationFromXVector HitNormal))
  (Actor|DestroyActor))

(fn ConstructionScript)