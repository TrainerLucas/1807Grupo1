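; Actor component that opens the start user interface and hands control over to it.
; OpenUserInterface creates the User_Interface_Start widget, stores it as DialogueWidget and adds it to the viewport.
; It then switches the first player to UI-only input with a visible cursor and disables movement on the BP_ThirdPersonCharacter.
; The component has no closing or restore logic, and its event graph is empty.
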(event EventBeginPlay)

(event EventTick
  (params (DeltaSeconds :type Float%20%28single-precision%29)))

(fn OpenUserInterface
  (bind _returnvalue (Game|GetPlayerController 0))
  (bind _returnvalue_2 (UserInterface|CreateWidget "/Game/Carpeta_De-Aidan/User_Interface_Start.User_Interface_Start_C" (Game|GetPlayerController 0)))
  (bind _output_get (Variables|Default|SetDialogueWidget _returnvalue_2))
  (UserInterface|Viewport|AddtoViewport _output_get 0)
  (Input|SetInputModeUIOnly _returnvalue _output_get "DoNotLock" false)
  (Variables|/Script/Engine.PlayerController|SetbShowMouseCursor _returnvalue true)
  (bind _asbp_third_person_character (Utilities|Casting|CastToBP_ThirdPersonCharacter (Game|GetPlayerCharacter 0)))
  (Pawn|Components|CharacterMovement|DisableMovement (Variables|/Script/Engine.Character|GetCharacterMovement _asbp_third_person_character)))